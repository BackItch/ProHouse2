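; Player character for an in-game building editor, with flying movement and Z cycling wall-opening, wall-material and floor-node edit modes.
; Each tick it finds the closest BooleanFloor by camera trace or nearest spline point, using screen-space distances for snap states and debug-drawn cues.
; Clicks add or remove floor nodes, send interact messages or remove openings.
; Shift toggles an inspection HUD, the mouse wheel adjusts inspected wall height, and key 1 saves floors.
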(event `InputAxis|Walk Forward`
  (params (AxisValue :type "Float (single-precision)"))
  ;[1 1 1] Movement
  (`self.AddMovementInput` (`self.GetActorForwardVector`) AxisValue))

(event `InputAxis|Turn`
  (params (AxisValue :type "Float (single-precision)"))
  ;[1 1 1] Movement
  (if (`PlayerController.bShowMouseCursor` (`GameplayStatics.GetPlayerController` 0))
    _
    (else
      _))
  (`self.AddControllerYawInput` AxisValue))

(event `InputAxis|LookUp`
  (params (AxisValue :type "Float (single-precision)"))
  ;[1 1 1] Movement
  (if (`PlayerController.bShowMouseCursor` (`GameplayStatics.GetPlayerController` 0))
    _
    (else
      _))
  (`self.AddControllerPitchInput` AxisValue))

(event `InputAxis|FlyUp`
  (params (AxisValue :type "Float (single-precision)"))
  ;[1 1 1] Movement
  (`self.AddMovementInput` (`self.GetActorUpVector`) AxisValue true))

(event `InputAxis|Strafe Right`
  (params (AxisValue :type "Float (single-precision)"))
  ;[1 1 1] Movement
  (`self.AddMovementInput` (`self.GetActorRightVector`) AxisValue true))

(event `Key|Z`
  (params (Key :type "Key Structure"))
  ;[1 1 1] Change Mode
  (:`Pressed`
    (`|MultiGate` false true
      (:`Out 0`
        (set `self.Edit Mode` "NewEnumerator1"))
      (:`Out 1`
        (set `self.Edit Mode` "NewEnumerator2"))
      (:`Out 2`
        (set `self.Edit Mode` "NewEnumerator0")))))

(event `Find Closest Floor Section`
  (bind _returnvalue (`GameplayStatics.GetPlayerCameraManager` 0))
  (bind _returnvalue_2 (`self.K2_GetActorLocation` _returnvalue))
  ;[1 1 1] Find Closest Floor Section
  (bind _outhit (`KismetSystemLibrary.LineTraceSingle` _returnvalue_2 (+ _returnvalue_2 (* (`self.GetActorForwardVector` _returnvalue) 50000)) "TraceTypeQuery1"))
  (bind (_bblockinghit _binitialoverlap _time _distance _location _impactpoint _normal _impactnormal _physmat _hitactor) (`GameplayStatics.BreakHitResult` _outhit))
  ;;[1 1 1] If we're looking directly at a floor. Easy. Set it as the closest.
  (bind _asboolean_floor (cast `/Game/BooleanFloor` _hitactor)
    (:`then`
      (set `self.Floor Section Closest` _asboolean_floor)
      (set `/Game/BooleanFloor.Am I being looked at?` true _asboolean_floor))
    (:`CastFailed`
      ;;[1 1 1] If we're looking directly at a wall, get the owning floor and set it.
      (bind _asboolean_piece (cast `/Game/BooleanPiece` _hitactor)
        (:`then`
          (bind _belongs_to_floor (`/Game/BooleanWall.Belongs to Floor` (`/Game/BooleanPiece.Piece of wall` _asboolean_piece)))
          (set `self.Floor Section Closest` _belongs_to_floor)
          (set `/Game/BooleanFloor.Am I being looked at?` true _belongs_to_floor))
        (:`CastFailed`
          (bind _asmy_game_mode (cast `/Game/MyGameMode` (`GameplayStatics.GetGameMode`))) ; Otherwise, do more complicated stuff to find the closest floor
          (set `self.Smallest Distance So Far` 10000000000.0)
          (set `self.LocalIndex` -1)
          (bind _floors (`/Game/MyGameMode.Floors` _asmy_game_mode))
          (for (_array_element _array_index) _floors
            (set `/Game/BooleanFloor.Am I being looked at?` false _array_element)
            (bind _floorspline (`/Game/BooleanFloor.FloorSpline` _array_element))
            (for _index (range (`SplineComponent.GetNumberOfSplinePoints` _floorspline))
              (bind _returnvalue_3 (`KismetMathLibrary.Vector_Distance` (`SplineComponent.GetLocationAtSplinePoint` _floorspline _index "World") (`/Game/BooleanFloor.Looking at on Plane` _array_element)))
              (if (< _returnvalue_3 (`self.Smallest Distance So Far`))
                (set `self.Smallest Distance So Far` _returnvalue_3)
                (set `self.LocalIndex` _array_index))))
          (bind _output (`|GetArrayItem` _floors (`self.LocalIndex`)))
          (set `/Game/BooleanFloor.Am I being looked at?` true _output)
          (set `self.Floor Section Closest` _output))))))

(event `Key|R`
  (params (Key :type "Key Structure"))
  (bind _test (`self.Test`))
  (:`Pressed`
    (`/Engine/EditorBlueprintResources/StandardMacros.IncrementInt` _test
      (:`  `
        (`KismetSystemLibrary.PrintString` (`KismetStringLibrary.Conv_IntToString` _test) :!label _label)
        (`KismetSystemLibrary.PrintString` (`KismetStringLibrary.Conv_IntToString` (`/Game/BooleanFloor.WrapValueAround` (`self.Floor Section Closest`) (`self.Test`) 4)) true true (struct :`R` 1.0 :`G` 0.009923 :`B` 0.03977 :`A` 1.0))))))

(event `Key|T`
  (params (Key :type "Key Structure"))
  (:`Pressed`
    (`/Engine/EditorBlueprintResources/StandardMacros.DecrementInt` (`self.Test`)
      (:`  `
        (goto _label)))))

(event `self.ReceiveTick`
  (params (DeltaSeconds :type "Float (single-precision)"))
  (bind _returnvalue (`GameplayStatics.GetPlayerController` 0))
  (bind _returnvalue_2 (`GameplayStatics.GetPlayerController` 0))
  (bind _location_of_nearest_spline_point (`self.Find Spline Point Locations`))
  (bind _returnvalue_3 (`GameplayStatics.GetPlayerController` 0))
  (bind _is_looking_at_node_ (`self.Is Looking at Node?`))
  (bind _floor_section_closest (`self.Floor Section Closest`))
  (bind _looking_at_on_plane (`/Game/BooleanFloor.Looking at on Plane` (`self.Floor Section Closest`)))
  (bind _floorspline (`/Game/BooleanFloor.FloorSpline` _floor_section_closest))
  (bind _looking_at_on_plane_2 (`/Game/BooleanFloor.Looking at on Plane` (`self.Floor Section Closest`)))
  (`|ExecutionSequence`
    (:`then_0`
      (`self.LookAt`)
      ;[1 1 1] Figure things out
      ;;[1 1 1] If Dragging, Don't try to figure out
      (if (not (`self.Is Dragging a Node?`))
        (`self.Find Closest Floor Section`)
        (`KismetSystemLibrary.DrawDebugLine` _location_of_nearest_spline_point _looking_at_on_plane_2 (struct :`R` 1.0 :`G` 0.983937 :`A` 1.0) 0.0 3.0)
        (set `self.Is Looking At Node?` (< (`KismetMathLibrary.Distance2D` (`GameplayStatics.ProjectWorldToScreen` _returnvalue_2 _location_of_nearest_spline_point) (`GameplayStatics.ProjectWorldToScreen` _returnvalue_2 _looking_at_on_plane_2)) (`self.Distance to Snap`)))
        (set `self.Is Looking Near Spline?` (< (`KismetMathLibrary.Distance2D` (`GameplayStatics.ProjectWorldToScreen` _returnvalue (`/Game/BooleanFloor.Looking at on Plane` (`self.Floor Section Closest`))) (`GameplayStatics.ProjectWorldToScreen` _returnvalue (`.Location Closest to World Location` (`self.Find Spline Point Locations`)))) (`self.Distance to Spline View`)))
        (set `self.Is Looking at Middle of Section?` (< (`KismetMathLibrary.Distance2D` (`GameplayStatics.ProjectWorldToScreen` _returnvalue_3 (`/Game/BooleanFloor.Find Location Closest to Input Key` _floor_section_closest (+ (`KismetMathLibrary.Conv_IntToDouble` (`KismetMathLibrary.FFloor` 0.0)) 0.5) _floorspline)) (`GameplayStatics.ProjectWorldToScreen` _returnvalue_3 (`/Game/BooleanFloor.Find Location Closest to Input Key` _floor_section_closest 0.0 _floorspline))) (`self.Distance to Snap`)))))
    (:`then_1`
      (if (and (`self.Is Looking Near Spline?`) (`|EnumEquality` (`self.Edit Mode`) "NewEnumerator0"))
        (`|ExecutionSequence`
          (:`then_0`
            (`KismetSystemLibrary.DrawDebugSphere` (`self.Find Spline Point Locations`) 10.0 12 (`KismetMathLibrary.SelectColor` (struct :`R` 0.068249 :`G` 0.885417 :`B` 0.160052 :`A` 1.0) (struct :`R` 0.911458 :`G` 0.742879 :`B` 0.057547 :`A` 1.0) _is_looking_at_node_))
            (if (not _is_looking_at_node_)
              (`KismetSystemLibrary.DrawDebugSphere` (`.Location Closest to World Location` (`self.Find Spline Point Locations`)) 12.0 16 (struct :`R` 0.144289 :`G` 0.293592 :`B` 0.520833 :`A` 1.0) 0.0 0.2))))))
    (:`then_2`
      (if (and (`self.Is Looking at Middle of Section?`) (not (`self.Is Looking At Node?`)) (`|EnumEquality` (`self.Edit Mode`) "NewEnumerator0"))
        (`KismetSystemLibrary.DrawDebugCylinder` (0.0 0.0 0.0) (0.0 0.0 0.0) 20.0 24 (struct :`R` 0.744792 :`G` 0.703665 :`B` 0.038791 :`A` 1.0) 0.0 2.0)
        (elif (and (`self.Is Looking at Opening?`) (`|EnumEquality` (`self.Edit Mode`) "NewEnumerator1"))
          (`KismetSystemLibrary.DrawDebugSphere` (`self.Opening Looking At`) 10.0 12 (struct :`G` 0.102902 :`B` 0.401042 :`A` 1.0)))))
    (:`then_3`
      (`KismetSystemLibrary.DrawDebugArrow` (+ _looking_at_on_plane (0.0 0.0 100.0)) _looking_at_on_plane 20.0 (struct) 0.0 5.0))))

(event `Key|LeftShift`
  (params (Key :type "Key Structure"))
  (bind _returnvalue (`GameplayStatics.GetPlayerCameraManager` 0))
  (bind _returnvalue_2 (`GameplayStatics.GetPlayerController` 0))
  (bind _returnvalue_3 (`GameplayStatics.GetPlayerCameraManager` 0))
  (bind (_bblockinghit _binitialoverlap _time _distance _location _impactpoint _normal _impactnormal _physmat _hitactor) (`GameplayStatics.BreakHitResult` (`self.Inspected Hit`)))
  (bind _returnvalue_4 (`self.K2_GetActorLocation` _returnvalue))
  (bind _returnvalue_5 (`self.K2_GetActorLocation` _returnvalue_3))
  ;[1 1 1] Shift: Inspect
  (:`Pressed`
    (if (`PlayerController.bShowMouseCursor` (`GameplayStatics.GetPlayerController` 0))
      (`self.Turn Off Hud`)
      (else
        (switch `/Game/EditingModeEnum` (`self.Edit Mode`)
          (:`NewEnumerator0`
            (bind (_outhit _returnvalue_6) (`KismetSystemLibrary.LineTraceSingle` :`Start` _returnvalue_4 :`End` (+ _returnvalue_4 (* (`self.GetActorForwardVector` _returnvalue) 50000)) :`TraceChannel` "TraceTypeQuery1" :`DrawDebugType` "ForDuration" :`DrawTime` 4.0))
            (set `self.Inspected Hit` _outhit))
          (:`NewEnumerator1`
            (bind _outhit_2 (`KismetSystemLibrary.LineTraceSingleForObjects` :`Start` _returnvalue_5 :`End` (+ _returnvalue_5 (* (`self.GetActorForwardVector` _returnvalue_3) 50000)) :`ObjectTypes` (`|MakeArray` "ObjectTypeQuery8" "ObjectTypeQuery9" :!type "EObjectTypeQuery Enum") :`DrawDebugType` "ForDuration" :`DrawTime` 4.0))
            (set `self.Inspected Hit` _outhit_2)))
        (if _returnvalue_6
          (message `/Game/Interface_Inspect.Inspect` _hitactor false)
          (`KismetSystemLibrary.PrintString` (`KismetStringLibrary.Concat_StrStr` "Inspect: " (`KismetSystemLibrary.GetDisplayName` _hitactor)))
          (set `self.LastInspected` _hitactor)
          (`self.Update Inspect HUD`)
          (set `PlayerController.bShowMouseCursor` true _returnvalue_2)
          (`Controller.SetIgnoreLookInput` _returnvalue_2 true))))))

(event `InputAction|LeftClick`
  (params (Key :type "Key Structure"))
  (bind _returnvalue (`GameplayStatics.GetPlayerCameraManager` 0))
  (bind _floor_section_dragged (`self.Floor Section Dragged`))
  (bind _returnvalue_2 (`self.K2_GetActorLocation` _returnvalue))
  ;[1 1 1] Left Click: Interact
  (:`Pressed`
    (`KismetSystemLibrary.PrintString` "click")
    (`|ExecutionSequence`
      (:`then_0`
        (if (`self.Is Looking at Node?`)
          _
          (elif (`self.Is Looking Near Spline?`)
            (if (not (`self.Is Looking at Middle of Section?`))
              (switch `/Game/EditingModeEnum` (`self.Edit Mode`)
                (:`NewEnumerator0`
                  (`/Game/BooleanFloor.Add New Spline Point` (`self.Floor Section Closest`))))))))
      (:`then_1`
        (bind _outhit (`KismetSystemLibrary.LineTraceSingleForObjects` :`Start` _returnvalue_2 :`End` (+ _returnvalue_2 (* (`self.GetActorForwardVector` _returnvalue) 50000)) :`ObjectTypes` (`|MakeArray` "ObjectTypeQuery8" "ObjectTypeQuery9" :!type "EObjectTypeQuery Enum") :`DrawDebugType` "ForDuration" :`DrawTime` 4.0))
        (bind (_bblockinghit _binitialoverlap _time _distance _location _impactpoint _normal _impactnormal _physmat _hitactor _hitcomponent) (`GameplayStatics.BreakHitResult` _outhit))
        (message `/Game/Interface_Clickable.Interact` _hitactor _hitcomponent _location)
        (`KismetSystemLibrary.PrintString` (`KismetStringLibrary.Concat_StrStr` "Clicked Actor: " (`KismetSystemLibrary.GetDisplayName` _hitactor)))
        (bind _asboolean_floor (cast `/Game/BooleanFloor` _hitactor))
        (set `self.Floor Section Dragged` _asboolean_floor))))
  (:`Released`
    (`/Engine/EditorBlueprintResources/StandardMacros.IsValid` _floor_section_dragged
      (:`Is Valid`
        (`/Game/BooleanFloor.Stop Dragging` _floor_section_dragged)
        (set `self.Is Dragging a Node?` false)))))

(event `Turn Off Hud`
  (bind _returnvalue (`GameplayStatics.GetPlayerController` 0))
  (`KismetSystemLibrary.PrintString` "Turn off hud")
  (set `PlayerController.bShowMouseCursor` false _returnvalue)
  (`Controller.ResetIgnoreInputFlags` _returnvalue)
  (`WidgetBlueprintLibrary.SetInputMode_GameOnly` _returnvalue)
  (`Widget.SetVisibility` (`self.WallInspectHud`) "Hidden"))

(event `Update Inspect HUD`
  (bind _returnvalue (`GameplayStatics.GetPlayerController` 0))
  (bind _returnvalue_2 (`KismetSystemLibrary.DoesImplementInterface` (`self.LastInspected`) "/Game/Interface_Inspect.Interface_Inspect_C"))
  ;[1 1 1] Inspect Hud
  (if (`KismetSystemLibrary.IsValid` (`self.WallInspectHud`))
    (if _returnvalue_2
      (`Widget.SetVisibility` (`self.WallInspectHud`) "Visible")
      (`WidgetBlueprintLibrary.SetInputMode_GameAndUIEx` _returnvalue null :!label _label_2)
      (else
        (`self.Turn Off Hud` :!label _label_3)))
    (elif _returnvalue_2
      (bind _returnvalue_3 (`|CreateWidget` "/Game/DebugWidget.DebugWidget_C" _returnvalue))
      (bind _output_get (set `self.WallInspectHud` _returnvalue_3))
      (`UserWidget.AddToViewport` _output_get 0)
      (goto _label_2)
      (else
        (goto _label_3)))))

(event `InputAction|RightClick`
  (params (Key :type "Key Structure"))
  (bind _returnvalue (`GameplayStatics.GetPlayerCameraManager` 0))
  (bind _returnvalue_2 (`self.K2_GetActorLocation` _returnvalue))
  ;[1 1 1] Right Click: Remove
  (:`Pressed`
    (switch `/Game/EditingModeEnum` (`self.Edit Mode`)
      (:`NewEnumerator0`
        (if (`self.Is Looking at Node?`)
          (`/Game/BooleanFloor.Remove Node` (`self.Floor Section Closest`))))
      (:`NewEnumerator1`
        (bind _outhit (`KismetSystemLibrary.LineTraceSingleForObjects` :`Start` _returnvalue_2 :`End` (+ _returnvalue_2 (* (`self.GetActorForwardVector` _returnvalue) 50000)) :`ObjectTypes` (`|MakeArray` "ObjectTypeQuery8" "ObjectTypeQuery9" :!type "EObjectTypeQuery Enum") :`DrawDebugType` "ForDuration" :`TraceColor` (struct :`R` 1.0 :`G` 0.739149 :`A` 1.0) :`DrawTime` 20.0))
        (bind _asopening_box (cast `/Game/OpeningBox` (`.HitActor` (`GameplayStatics.BreakHitResult` _outhit))))
        (`/Game/OpeningBox.Remove` _asopening_box)))))

(event `LookAt`
  (bind _returnvalue (`GameplayStatics.GetPlayerCameraManager` 0))
  (bind _returnvalue_2 (`self.K2_GetActorLocation` _returnvalue))
  ;[1 1 1] Look At
  (bind _outhit (`KismetSystemLibrary.LineTraceSingleForObjects` :`Start` _returnvalue_2 :`End` (+ _returnvalue_2 (* (`self.GetActorForwardVector` _returnvalue) 50000)) :`ObjectTypes` (`|MakeArray` "ObjectTypeQuery8" :!type "EObjectTypeQuery Enum") :`DrawTime` 1.0))
  (bind (_bblockinghit _binitialoverlap _time _distance _location _impactpoint _normal _impactnormal _physmat _hitactor _hitcomponent) (`GameplayStatics.BreakHitResult` _outhit))
  (message `/Game/Interface_LookAt.LookAt` _hitactor _hitcomponent _location))

(event `Key|MouseScrollUp`
  (params (Key :type "Key Structure"))
  (bind (_asboolean_piece _bsuccess) (cast `/Game/BooleanPiece` (`self.LastInspected`) :!pure true))
  (bind _piece_of_wall (`/Game/BooleanPiece.Piece of wall` _asboolean_piece))
  (bind _output (`|GetArrayItem` (`/Game/BooleanFloor.Wall Info` (`/Game/BooleanWall.Belongs to Floor` _piece_of_wall)) (`/Game/BooleanWall.Belongs to Floor Node` _piece_of_wall)))
  (:`Pressed`
    (if _bsuccess
      (set `self.New Wall Height` (+ (`.WallHeightinFeet_11_525F97704B24114D85762EACD413A6C9` (break `/Game/WallStruct` _output)) 1.0))
      (bind _structout (setmembers `/Game/WallStruct` :`StructRef` _output :`SectionHasWall` false :`Wall Height (in Feet)` (`self.New Wall Height`)))
      (bind (_sectionhaswall _wallheightinfeet _interiormaterial _openingsinwall _triggersphereref _wallref) (break `/Game/WallStruct` _structout))
      (`KismetSystemLibrary.PrintString` (`KismetStringLibrary.Conv_DoubleToString` _wallheightinfeet))
      (`/Game/BooleanWall.Refresh Wall` _wallref))))

(event `Key|MouseScrollDown`
  (params (Key :type "Key Structure"))
  (bind (_asboolean_piece _bsuccess) (cast `/Game/BooleanPiece` (`self.LastInspected`) :!pure true))
  (bind _piece_of_wall (`/Game/BooleanPiece.Piece of wall` _asboolean_piece))
  (bind _output (`|GetArrayItem` (`/Game/BooleanFloor.Wall Info` (`/Game/BooleanWall.Belongs to Floor` _piece_of_wall)) (`/Game/BooleanWall.Belongs to Floor Node` _piece_of_wall)))
  (:`Pressed`
    (if _bsuccess
      (bind _structout (setmembers `/Game/WallStruct` :`StructRef` _output :`Wall Height (in Feet)` (+ (`.WallHeightinFeet_11_525F97704B24114D85762EACD413A6C9` (break `/Game/WallStruct` _output)) -1.0)))
      (bind (_sectionhaswall _wallheightinfeet _interiormaterial _openingsinwall _triggersphereref _wallref) (break `/Game/WallStruct` _structout))
      (`KismetSystemLibrary.PrintString` (`KismetStringLibrary.Conv_DoubleToString` _wallheightinfeet))
      (`/Game/BooleanWall.Refresh Wall` _wallref))))

(event `Key|One`
  (params (Key :type "Key Structure"))
  (:`Pressed`
    (bind _asmy_game_instance (cast `/Game/MyGameInstance` (`GameplayStatics.GetGameInstance`)))
    (bind _outactors (`GameplayStatics.GetAllActorsOfClass` "/Game/BooleanFloor.BooleanFloor_C"))
    (bind _savegamedata (`/Game/MyGameInstance.SaveGameData` _asmy_game_instance))
    (set `/Game/MySaveGameObject.Floors` _outactors _savegamedata)
    (bind _returnvalue (`GameplayStatics.SaveGameToSlot` _savegamedata (`/Game/MyGameInstance.SaveSlotName` _asmy_game_instance)))
    (if _returnvalue
      (`KismetSystemLibrary.PrintString` "********* Saved")
      (else
        (`KismetSystemLibrary.PrintString` "Something went wrong Saving. Should never happen")))))

(event `Key|Two`
  (params (Key :type "Key Structure"))
  (:`Pressed`
    (cast `/Game/MyGameInstance` (`GameplayStatics.GetGameInstance`))))

(fn `Find Spline Point Locations`
  (returns (`Location of Nearest Spline Point` :type "Vector Structure") (`Location Closest to World Location` :type "Vector Structure") (`Node Closest` :type Integer))
  (bind _floor_section_closest (`self.Floor Section Closest`))
  (bind _floorspline (`/Game/BooleanFloor.FloorSpline` _floor_section_closest))
  (bind _looking_at_on_plane (`/Game/BooleanFloor.Looking at on Plane` _floor_section_closest))
  (bind _returnvalue (`KismetMathLibrary.Round` (`SplineComponent.FindInputKeyClosestToWorldLocation` _floorspline _looking_at_on_plane)))
  (return (`SplineComponent.GetLocationAtSplinePoint` _floorspline _returnvalue "World") (`SplineComponent.FindLocationClosestToWorldLocation` _floorspline _looking_at_on_plane "World") _returnvalue))

(fn `UserConstructionScript`)